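; AGM-65 missile Blueprint that adds fin-driven pitch and yaw flight dynamics to its parent missile class.
; UpdateMissileMotion integrates angular velocity and rotation from fin angles, gains, inertia and deflection-dependent damping, prints debug values, then calls the parent.
; UpdateWingDeg advances both fin angles and mirrors opposing fins on the anim instance.
; It runs only once at BeginPlay, since its Tick call is disconnected.
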(event `self.ReceiveBeginPlay`
  (bind _asbpa_west_missile_agm65 (cast `/Game/VigilanteContent/Projectiles/West_Missile_AGM65/BPA_West_Missile_AGM65` (`SkeletalMeshComponent.GetAnimInstance` (`self.SkeletalMesh`))))
  (set `self.Anim Instance` _asbpa_west_missile_agm65)
  (`self.Update Wing Deg` 1.0)
  (`parent.ReceiveBeginPlay`))

(event `self.ReceiveTick`
  (params (DeltaSeconds :type "Float (single-precision)"))
  (`parent.ReceiveTick` DeltaSeconds))

(fn `Update Missile Motion`
  (params (`Delta Time` :type "Float (double-precision)"))
  (locals (Kp :type "Float (double-precision)" :default 1.0) (Ky :type "Float (double-precision)" :default 1.0) (Dp :type "Float (double-precision)" :default 0.1) (Dy :type "Float (double-precision)" :default 0.1) (Iy :type "Float (double-precision)" :default 1.0) (Iz :type "Float (double-precision)" :default 1.0))
  (bind (_rot_vel_roll _rot_vel_pitch _rot_vel_yaw) (`KismetMathLibrary.BreakRotator` (`self.Rot Vel`)))
  (bind (_rotation_roll _rotation_pitch _rotation_yaw) (`KismetMathLibrary.BreakRotator` (`self.Rotation`)))
  (bind (_returnvalue_roll _returnvalue_pitch _returnvalue_yaw) (`KismetMathLibrary.BreakRotator` (* (`self.Rot Vel`) `Delta Time`)))
  (bind _output_get (set `self.Rot Vel` (`KismetMathLibrary.MakeRotator` 0.0 (+ (* (- (/ (* (`self.P Wing Deg`) (`local.Kp`)) (`local.Iy`)) (* (+ (`local.Dp`) (* (`KismetMathLibrary.Abs` (`self.P Wing Deg`)) 0.01)) _rot_vel_pitch)) `Delta Time`) _rot_vel_pitch) (+ (* (- (/ (* (`self.Y Wing Deg`) (`local.Ky`)) (`local.Iz`)) (* (+ (`local.Dy`) (* (`KismetMathLibrary.Abs` (`self.Y Wing Deg`)) 0.01)) _rot_vel_yaw)) `Delta Time`) _rot_vel_yaw))))
  (set `self.Rotation` (`KismetMathLibrary.MakeRotator` (+ _rotation_roll _returnvalue_roll) (+ _rotation_pitch _returnvalue_pitch) (+ _rotation_yaw _returnvalue_yaw)))
  (`KismetSystemLibrary.PrintString` (`KismetStringLibrary.Concat_StrStr` "P Rot Vel: " (`KismetStringLibrary.Conv_DoubleToString` (.pitch _output_get)) " Y Rot Vel: " (`KismetStringLibrary.Conv_DoubleToString` (.yaw _output_get)) " P Wing Deg: " (`KismetStringLibrary.Conv_DoubleToString` (`self.P Wing Deg`)) " Y Wing Deg: " (`KismetStringLibrary.Conv_DoubleToString` (`self.Y Wing Deg`))) true true (struct :`R` 1.0 :`G` 0.116979 :`B` 0.230721 :`A` 1.0) 20.0)
  (`parent.Update Missile Motion` `Delta Time`))

(fn `UserConstructionScript`
  (`parent.UserConstructionScript`))